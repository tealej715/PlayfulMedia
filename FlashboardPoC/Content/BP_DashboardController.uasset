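; Dashboard controller Blueprint that exposes setter functions for the speed and colour scheme of a dashboard display.
; Each function writes its value straight into the MPC_Global Material Parameter Collection, so any material reading that collection picks up the change.
; SetThemeTertiary writes ThemeColourQuaternary and SetThemeQuaternary overwrites ThemeColourPrimary, so no setter here writes a tertiary parameter.
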(event `self.ReceiveBeginPlay`)

(fn `SetSpeed`
  (params (Value :type "Float (double-precision)"))
  (`KismetMaterialLibrary.SetScalarParameterValue` "/Game/Collections/MPC_Global.MPC_Global" "CurrentSpeed" Value))

(fn `SetTextPrimary`
  (params (Value :type "LinearColor Structure"))
  (`KismetMaterialLibrary.SetVectorParameterValue` "/Game/Collections/MPC_Global.MPC_Global" "TextColourPrimary" Value))

(fn `SetTextSecondary`
  (params (Value :type "LinearColor Structure"))
  (`KismetMaterialLibrary.SetVectorParameterValue` "/Game/Collections/MPC_Global.MPC_Global" "TextColourSecondary" Value))

(fn `SetThemePrimary`
  (params (Value :type "LinearColor Structure"))
  (`KismetMaterialLibrary.SetVectorParameterValue` "/Game/Collections/MPC_Global.MPC_Global" "ThemeColourPrimary" Value))

(fn `SetThemeQuaternary`
  (params (Value :type "LinearColor Structure"))
  (`KismetMaterialLibrary.SetVectorParameterValue` "/Game/Collections/MPC_Global.MPC_Global" "ThemeColourPrimary" Value))

(fn `SetThemeSecondary`
  (params (Value :type "LinearColor Structure"))
  (`KismetMaterialLibrary.SetVectorParameterValue` "/Game/Collections/MPC_Global.MPC_Global" "ThemeColourSecondary" Value))

(fn `SetThemeTertiary`
  (params (Value :type "LinearColor Structure"))
  (`KismetMaterialLibrary.SetVectorParameterValue` "/Game/Collections/MPC_Global.MPC_Global" "ThemeColourQuaternary" Value))

(fn `UserConstructionScript`)